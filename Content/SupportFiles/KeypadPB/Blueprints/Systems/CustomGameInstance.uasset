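; Game instance that acts as a shared hub for UI, session state and player-facing helper events in the keypad project.
; Creates and tracks splash, main menu, ESC and player menu widgets, toggles the player menu by FlipFlop, and adds log entries to it.
; Also loads the prototype level, forwards inventory additions, blends the camera back to the player and runs a timed O2 breathing flag.
; The exit screen reference is set to None rather than the created widget.
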(event Custom|Ability:%20O2%20Tank
  (Variables|Default|SetAllow%20Temp%20Breathing false)
  (Utilities|FlowControl|Delay 1e+01)
  (Variables|Default|SetAllow%20Temp%20Breathing true))

(event Custom|Add%20To%20Inventory
  (params (Object%20Type :type Byte))
  (CallFunction|AddtoInventory Object%20Type))

(event Custom|Add%20Character%20Reference
  (params (player%20character :type %20Object%20Reference))
  (Variables|Default|SetPlayer%20character 0))

(event Custom|Show%20ESC%20Menu
  ;[1 1 1] Show ESC menu
  (bind _returnvalue (UserInterface|CreateWidget 0))
  (Variables|UI|SetESC%20Widget _returnvalue)
  (UserInterface|Viewport|AddtoViewport _returnvalue 0)
  (Variables|/Script/Engine.PlayerController|SetbShowMouseCursor (Game|GetPlayerController 0) true))

(event Custom|Set%20Camera
  ;[1 1 1] Change Camera to player
  (Game|Player|SetViewTargetwithBlend (Game|GetPlayerController 0) (Game|GetPlayerCharacter 0) 0.5 "VTBlend_EaseInOut" 1.0 false)
  (CallFunction|SetMouseVisability))

(event Custom|Display%20UI%20to%20Screen
  (params (Data :type %20Structure))
  (bind _returnvalue (UserInterface|CreateWidget 0 0 Data))
  (UserInterface|Viewport|AddtoViewport _returnvalue 0)
  (CallFunction|SetMouseVisability))

(event Custom|Toggle%20Player%20Menu
  (bind _player_menu_ui (Variables|UI|GetPlayer%20Menu%20UI))
  (Utilities|FlowControl|FlipFlop
    (:A
      (Widget|SetVisibility _player_menu_ui "Visible")
      (CallFunction|SetMouseVisability(UIOnly) "NewEnumerator0" _player_menu_ui)
      (Variables|Default|SetVisable true))
    (:B
      (Widget|SetVisibility _player_menu_ui "Hidden")
      (CallFunction|SetMouseVisability(UIOnly) "NewEnumerator0" _player_menu_ui))))

(event Custom|Initialize%20UI
  (bind _returnvalue (UserInterface|CreateWidget "/CustomUtilities/UI/Player/PlayerHUD.PlayerHUD_C"))
  (bind _output_get (Variables|UI|SetPlayer%20Menu%20UI _returnvalue))
  (UserInterface|Viewport|AddtoViewport _returnvalue 0)
  (Widget|SetVisibility _output_get "Hidden"))

(event Custom|Reference%20landscape
  (params (landscape :type Landscape%20Object%20Reference))
  (Variables|Default|Setlandscape landscape))

(fn AddEntrytoLogUI
  (params (Data%20Struct :type %20Structure))
  (bind _player_menu_ui (Variables|UI|GetPlayer%20Menu%20UI))
  (bind _loguimenu (Variables|Default|GetLogUIMenu _player_menu_ui))
  (bind _returnvalue (UserInterface|CreateWidget 0 (Game|GetPlayerController 0) Data%20Struct))
  (Utilities|IsValid _loguimenu
    (:Is%20Valid
      (Widget|Panel|AddChild (Variables|Default|GetContentsBox _loguimenu) _returnvalue))))

(event Custom|Show%20Splash%20Screen
  ;[1 1 1] Show Splash Screen
  (bind _returnvalue (UserInterface|CreateWidget 0))
  (Variables|UI|SetSplash%20Screen%20UI _returnvalue)
  (UserInterface|Viewport|AddtoViewport _returnvalue 0))

(event Custom|Program%20EXE%20Started
  ;[1 1 1] Program Started
  (Variables|System|SetGame%20EXE%20Started true))

(event Custom|Show%20Exit%20Screen
  ;[1 1 1] Show Exit Screen
  (bind _returnvalue (UserInterface|CreateWidget 0))
  (bind _output_get (Variables|UI|SetExit%20Menu%20UI 0 _returnvalue))
  (UserInterface|Viewport|AddtoViewport _output_get 0))

(event Custom|Show%20Main%20menu
  ;[1 1 1] Show Main Menu
  (bind _returnvalue (UserInterface|CreateWidget 0 (Game|GetPlayerController 0)))
  (Variables|UI|SetMain%20Menu%20UI _returnvalue)
  (UserInterface|Viewport|AddtoViewport _returnvalue 0))

(event Custom|Load%20Main%20Level
  ;[1 1 1] Load main level
  (Game|OpenLevel(byName) "PrototypeLevel001_2")
  (Variables|System|SetIn%20Game%20Session true))